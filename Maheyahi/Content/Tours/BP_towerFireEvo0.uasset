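; Base-tier fire tower actor for tower defense that configures its mesh, range and fire rate from the StatsTours data table.
; Tick calls Shoot when a target is valid, spawning an actor given that target, then reloading via a delay.
; Otherwise it runs a throttled sphere trace for the closest pawn, alongside range-sphere overlap events.
; Cast classes and target assignments are unresolved, with enemy logic marked as pending.
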(event OnComponentBeginOverlap(Sphere)
  (params (OverlappedComponent :type Primitive%20Component%20Object%20Reference) (OtherActor :type Actor%20Object%20Reference) (OtherComp :type Primitive%20Component%20Object%20Reference) (OtherBodyIndex :type Integer) (bFromSweep :type Boolean) (SweepResult :type Hit%20Result%20Structure%20%28by%20ref%29))
  (Utilities|IsValid (.Towertarget (Variables|Default|GetTowertarget))
    (:Is%20Not%20Valid
      (bind _asennemies (Utilities|Casting|CastTo OtherActor))
      (Variables|Default|SetTowertarget "" _asennemies))))

(event OnComponentEndOverlap(Sphere)
  (params (OverlappedComponent :type Primitive%20Component%20Object%20Reference) (OtherActor :type Actor%20Object%20Reference) (OtherComp :type Primitive%20Component%20Object%20Reference) (OtherBodyIndex :type Integer))
  (if (== 0 OtherActor)
    (Variables|Default|SetTowertarget "")))

(event Custom|TowerInit
  (bind _towerstruct (Variables|Default|GetTowerStruct))
  (bind (_nom _portée _degats _firerate _mesh) (Utilities|Struct|BreakTowerStruct _towerstruct))
  (Components|StaticMesh|SetStaticMesh (Variables|Mesh|GetStaticMesh) _mesh)
  (Components|Sphere|SetSphereRadius (Variables|Default|GetSphere) _portée true))

(event Custom|shoot
  ;[1 1 1] Modifier quand il y aura les ennemis
  (Variables|Default|Setreload true)
  (Game|SpawnActorfromClass 0 (Transformation|GetActorTransform) "AlwaysSpawn" 0 (.Towertarget (Variables|Default|GetTowertarget)) 0)
  (Utilities|FlowControl|Delay (.firerate (Utilities|Struct|BreakTowerStruct (Variables|Default|GetTowerStruct))))
  (Variables|Default|Setreload false))

(event Custom|SelectNewTarget
  (bind _returnvalue (Transformation|GetActorLocation))
  (Variables|Default|SetCheckForTarget true)
  (bind _outhits (Collision|MultiSphereTraceForObjects _returnvalue (- _returnvalue "0, 0, 0") (.Portée (Utilities|Struct|BreakTowerStruct (Variables|Default|GetTowerStruct))) (Utilities|Array|MakeArray "ObjectTypeQuery3") false 0 "None"))
  (if true
    (bind _target (CallFunction|CloserTarget 0 _outhits))
    (Utilities|IsValid _target
      (:Is%20Valid
        (Variables|Default|SetTowertarget "" _target))
      (:Is%20Not%20Valid
        _)))
  (Utilities|FlowControl|Delay 0.2)
  (Variables|Default|SetCheckForTarget false))

(event EventBeginPlay
  (bind _returnvalue (Utilities|GetDataTableRow "/Game/Tours/StatsTours.StatsTours" "Chair_Feu")
    (:then
      (Variables|Default|SetTowerStruct _returnvalue)
      (CallFunction|TowerInit))))

(event EventTick
  (params (DeltaSeconds :type Float%20%28single-precision%29))
  (Utilities|IsValid (.Towertarget (Variables|Default|GetTowertarget))
    (:Is%20Valid
      (if (not (Variables|Default|Getreload))
        (CallFunction|Shoot)))
    (:Is%20Not%20Valid
      (if (not (Variables|Default|GetCheckForTarget))
        (CallFunction|SelectNewTarget)))))

(fn ConstructionScript)

(fn CloserTarget
  (params (Array :type Array%20of%20Hit%20Result%20Structures))
  ;[1 1 1] Modifier quand il y aura les ennemis
  (for _array_element Array
    (bind _asennemies (Utilities|Casting|CastTo (.HitActor (Collision|BreakHitResult _array_element))))
    (Utilities|IsValid (Variables|Default|GetIsATarget?)
      (:Is%20Valid
        (if (< (Math|Vector|VectorLength (- (Transformation|GetActorLocation) (Transformation|GetActorLocation (.HitActor (Collision|BreakHitResult _array_element))))) (Variables|Default|GetDinstanceTemp))
          (Variables|Default|SetIsATarget? _asennemies)
          (Variables|Default|SetDinstanceTemp (Math|Vector|VectorLength (- (Transformation|GetActorLocation) (Transformation|GetActorLocation (.HitActor (Collision|BreakHitResult _array_element))))))))
      (:Is%20Not%20Valid
        (Variables|Default|SetIsATarget? _asennemies)
        (Variables|Default|SetDinstanceTemp (Math|Vector|VectorLength (- (Transformation|GetActorLocation) (Transformation|GetActorLocation (.HitActor (Collision|BreakHitResult _array_element)))))))))
  (return (Variables|Default|GetIsATarget?)))