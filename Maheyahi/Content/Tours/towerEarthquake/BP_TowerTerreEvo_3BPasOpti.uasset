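; Earth (Earthquake) tower evolution 3B: loads stats from a data table and fires Projectile_Terre3B at the nearest listed enemy.
; Tick drives cooldown-gated shooting and retargeting, plus a scan throttled by a 0.5s delay that appends in-range enemies of seven classes to a never-cleared array.
; Clicking toggles a widget borrowed from the fire tower.
; Selling respawns the base tower, refunds SoulMoney and destroys this one.
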(event Custom|shoot
  (bind _returnvalue (Transformation|GetActorTransform))
  (bind _returnvalue_2 (Transformation|GetActorLocation))
  (bind _towerstruct (Variables|Default|GetTowerStruct))
  (bind (_nom _portée _degats _firerate) (Utilities|Struct|BreakTowerStruct _towerstruct))
  ;[1 1 1] Modifier quand il y aura les ennemis
  (Variables|Default|Setreload true)
  (Game|SpawnActorfromClass "/Game/Tours/towerEarthquake/Projectile_Terre3B.Projectile_Terre3B_C" (Math|Transform|MakeTransform (Math|Vector|MakeVector (.x _returnvalue_2) (.y _returnvalue_2) (+ (.z _returnvalue_2) 2e+02)) (.rotation _returnvalue) (.scale _returnvalue)) "AlwaysSpawn" 0 (Variables|Default|GetTowertarget) _degats 0)
  (Utilities|FlowControl|Delay _firerate)
  (Variables|Default|Setreload false))

(event Custom|SelectNewTarget
  (Variables|Default|SetCheckfortarget true)
  (CallFunction|CloserTarget2)
  (Utilities|FlowControl|Delay 0.2)
  (Variables|Default|SetCheckfortarget false))

(event Custom|sellTowerTerreEvo3b
  (bind _returnvalue (Transformation|GetActorTransform))
  ;[1 1 1] Sell tower terre evo 3b
  (Game|SpawnActorfromClass "/Game/Tours/BP_towerBase.BP_towerBase_C" (Math|Transform|MakeTransform (.location _returnvalue) (.rotation _returnvalue) "1,1,1") "Undefined" 0 0)
  (bind _astop_down_character (Utilities|Casting|CastToTopDownCharacter (Game|GetPlayerCharacter 0)))
  (Variables|/Game/TopDownBP/Blueprints/TopDownCharacter.TopDownCharacter_C|SetSoul_Money _astop_down_character (+ (Variables|/Game/TopDownBP/Blueprints/TopDownCharacter.TopDownCharacter_C|GetSoul_Money _astop_down_character) (Variables|/Game/TopDownBP/Blueprints/TopDownCharacter.TopDownCharacter_C|GetRevente_Tours1 _astop_down_character)))
  (Actor|DestroyActor)
  ;[1 1 1] Ouverture/fermeture du widget
  (Widget|RemovefromParent (stale MouseInput|EventActorOnClicked _returnvalue)))

(event EventBeginPlay
  (bind _returnvalue (Utilities|GetDataTableRow "/Game/Tours/StatsTours.StatsTours" "Earthquake_Tower3B")
    (:then
      (Variables|Default|SetTowerStruct _returnvalue))))

(event MouseInput|EventActorOnClicked
  (params (ButtonPressed :type Key%20Structure :default "None"))
  ;[1 1 1] Ouverture/fermeture du widget
  (Utilities|FlowControl|FlipFlop
    (:A
      (bind _returnvalue (UserInterface|CreateWidget "/Game/Tours/towerFire/widgetTowerFireEvo1.widgetTowerFireEvo1_C"))
      (UserInterface|Viewport|AddtoViewport _returnvalue 0))
    (:B
      (Widget|RemovefromParent _returnvalue))))

(event EventTick
  (params (DeltaSeconds :type Float%20%28single-precision%29))
  (Utilities|FlowControl|Sequence
    (:then_0
      (if (Utilities|IsValid (Variables|Default|GetTowertarget))
        (if (not (Variables|Default|Getreload))
          (CallFunction|Shoot)
          (if (Utilities|IsValid (Variables|Default|GetTowertarget))
            (Variables|Default|SetTowertarget (Variables|Default|GetNoneTarget))
            (CallFunction|SelectNewTarget :!label _label)))
        (elif (not (Variables|Default|GetCheckForTarget))
          (goto _label))))
    (:then_1
      (if (Variables|Default|GetLag)
        (Variables|Default|SetLag false)
        (bind _outactors (Actor|GetAllActorsOfClass "/Game/deplacement+vague/jomviking1.jomviking1_C"))
        (for _array_element _outactors
          (if (<= (Math|Vector|Distance(Vector) (Transformation|GetActorLocation _array_element) (Transformation|GetActorLocation)) (.portée (Variables|Default|GetTowerstruct)))
            (Utilities|Array|Add (Variables|Default|GetTableau%20Ennemis) _array_element)))
        (bind _outactors_2 (Actor|GetAllActorsOfClass "/Game/deplacement+vague/jomviking2.jomviking2_C"))
        (for _array_element_2 _outactors_2
          (if (<= (Math|Vector|Distance(Vector) (Transformation|GetActorLocation _array_element_2) (Transformation|GetActorLocation)) (.portée (Variables|Default|GetTowerstruct)))
            (Utilities|Array|Add (Variables|Default|GetTableau%20Ennemis) _array_element_2)))
        (bind _outactors_3 (Actor|GetAllActorsOfClass "/Game/deplacement+vague/cav1.cav1_C"))
        (for _array_element_3 _outactors_3
          (if (<= (Math|Vector|Distance(Vector) (Transformation|GetActorLocation _array_element_3) (Transformation|GetActorLocation)) (.portée (Variables|Default|GetTowerstruct)))
            (Utilities|Array|Add (Variables|Default|GetTableau%20Ennemis) _array_element_3)))
        (bind _outactors_4 (Actor|GetAllActorsOfClass "/Game/deplacement+vague/cav2.cav2_C"))
        (for _array_element_4 _outactors_4
          (if (<= (Math|Vector|Distance(Vector) (Transformation|GetActorLocation _array_element_4) (Transformation|GetActorLocation)) (.portée (Variables|Default|GetTowerstruct)))
            (Utilities|Array|Add (Variables|Default|GetTableau%20Ennemis) _array_element_4)))
        (bind _outactors_5 (Actor|GetAllActorsOfClass "/Game/deplacement+vague/berserker_1.berserker_1_C"))
        (for _array_element_5 _outactors_5
          (if (<= (Math|Vector|Distance(Vector) (Transformation|GetActorLocation _array_element_5) (Transformation|GetActorLocation)) (.portée (Variables|Default|GetTowerstruct)))
            (Utilities|Array|Add (Variables|Default|GetTableau%20Ennemis) _array_element_5)))
        (bind _outactors_6 (Actor|GetAllActorsOfClass "/Game/deplacement+vague/berserker_2.berserker_2_C"))
        (for _array_element_6 _outactors_6
          (if (<= (Math|Vector|Distance(Vector) (Transformation|GetActorLocation _array_element_6) (Transformation|GetActorLocation)) (.portée (Variables|Default|GetTowerstruct)))
            (Utilities|Array|Add (Variables|Default|GetTableau%20Ennemis) _array_element_6)))
        (bind _outactors_7 (Actor|GetAllActorsOfClass "/Game/deplacement+vague/BOSS.BOSS_C"))
        (for _array_element_7 _outactors_7
          (if (<= (Math|Vector|Distance(Vector) (Transformation|GetActorLocation _array_element_7) (Transformation|GetActorLocation)) (.portée (Variables|Default|GetTowerstruct)))
            (Utilities|Array|Add (Variables|Default|GetTableau%20Ennemis) _array_element_7)))
        (Utilities|FlowControl|Delay 0.5)
        (Variables|Default|SetLag true)))))

(fn ConstructionScript)

(fn CloserTarget
  (params (Array :type Array%20of%20Hit%20Result%20Structures))
  ;[1 1 1] Modifier quand il y aura les ennemis
  (for _array_element Array
    (bind _asjomviking_1 (Utilities|Casting|CastTojomviking1 (.HitActor (Collision|BreakHitResult _array_element))))
    (Utilities|IsValid (LocalVariables|GetIs%20a%20Target?)
      (:Is%20Valid
        (if (< (Math|Vector|VectorLength (- (Transformation|GetActorLocation) (Transformation|GetActorLocation (.HitActor (Collision|BreakHitResult _array_element))))) (Variables|Default|Getdistance%20temp))
          (LocalVariables|SetIs%20a%20Target? _asjomviking_1)
          (Variables|Default|Setdistance%20temp (Math|Vector|VectorLength (- (Transformation|GetActorLocation) (Transformation|GetActorLocation (.HitActor (Collision|BreakHitResult _array_element))))))))
      (:Is%20Not%20Valid
        (LocalVariables|SetIs%20a%20Target? _asjomviking_1)
        (Variables|Default|Setdistance%20temp (Math|Vector|VectorLength (- (Transformation|GetActorLocation) (Transformation|GetActorLocation (.HitActor (Collision|BreakHitResult _array_element)))))))))
  (return (LocalVariables|GetIs%20a%20Target?)))

(fn CloserTarget2
  (bind _output_get (Variables|Default|Setdistance%20temp 1e+06))
  (for _array_element (Variables|Default|GetTableau%20Ennemis)
    (if (Utilities|IsValid _array_element)
      (if (<= (Math|Vector|Distance(Vector) (Transformation|GetActorLocation _array_element) (Transformation|GetActorLocation)) _output_get)
        (Variables|Default|Setdistance%20temp (Math|Vector|Distance(Vector) (Transformation|GetActorLocation _array_element) (Transformation|GetActorLocation)))
        (Variables|Default|SetTowertarget _array_element)))))