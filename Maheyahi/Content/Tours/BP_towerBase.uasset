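; BP_towerBase is a tower build spot that replaces itself with an earthquake, thunder or fire Evo0 tower.
; Each spawn event creates its tower at the actor's transform, then destroys the base.
; A build widget, toggled at BeginPlay, rotates toward the player character every Tick.
; Cube cursor events set materials, but hover-begin and click-to-toggle sit behind constant-condition branches that never run.
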(event OnBeginCursorOver(Cube)
  (params (TouchedComponent :type Primitive%20Component%20Object%20Reference))
  ;[1 1 1] Changement du matériel on hover
  (if (not true)
    (Rendering|Material|SetMaterial (Variables|Default|GetCube) 0 0)))

(event OnEndCursorOver(Cube)
  (params (TouchedComponent :type Primitive%20Component%20Object%20Reference))
  ;[1 1 1] Changement du matériel on hover
  (Rendering|Material|SetMaterial (Variables|Default|GetCube) 0 0))

(event OnClicked(Cube)
  (params (TouchedComponent :type Primitive%20Component%20Object%20Reference) (ButtonPressed :type Key%20Structure :default "None"))
  ;[1 0.9159 0.6242] Display widget on click
  (if (not true)
    (Rendering|ToggleVisibility (Variables|Default|GetwidgetTowerBuild) false)))

(event Custom|spawnTowerThunderEvo0
  (bind _returnvalue (Transformation|GetActorTransform))
  ;[0.3028 0.7537 1] TEMPLATE spawn tour de foudre Evo0
  (Game|SpawnActorfromClass "/Game/Tours/BP_towerThunderEvo0.BP_towerThunderEvo0_C" (Math|Transform|MakeTransform (.location _returnvalue) (.rotation _returnvalue) "1,1,1") "Undefined" 0 0)
  (Actor|DestroyActor))

(event Custom|spawnTowerFireEvo0
  (bind _returnvalue (Transformation|GetActorTransform))
  ;[1 0.5736 0.1421] TEMPLATE spawn tour de feu Evo0
  (Game|SpawnActorfromClass "/Game/Tours/BP_towerFireEvo0.BP_towerFireEvo0_C" (Math|Transform|MakeTransform (.location _returnvalue) (.rotation _returnvalue) "1,1,1") "Undefined" 0 0)
  (Actor|DestroyActor))

(event Custom|spawnTowerEarthquakeEvo0
  (bind _returnvalue (Transformation|GetActorTransform))
  ;[0.4552 0.37 0.09641] TEMPLATE spawn tour de terre Evo0
  (Game|SpawnActorfromClass "/Game/Tours/BP_towerEarthquakerEvo0.BP_towerEarthquakerEvo0_C" (Math|Transform|MakeTransform (.location _returnvalue) (.rotation _returnvalue) "1,1,1") "Undefined" 0 0)
  (Actor|DestroyActor))

(event EventTick
  (params (DeltaSeconds :type Float%20%28single-precision%29))
  ;[1 1 1] Orienter le widget face au personnage
  (Transformation|SetRelativeRotation (Variables|Default|GetwidgetTowerBuild) (Math|Rotator|FindLookatRotation (Transformation|GetActorLocation) (Transformation|GetActorLocation (Game|GetPlayerCharacter 0))) false false))

(event EventBeginPlay
  ;[1 0.9159 0.6242] Display widget on click
  (Rendering|ToggleVisibility (Variables|Default|GetwidgetTowerBuild) false))

(fn ConstructionScript)