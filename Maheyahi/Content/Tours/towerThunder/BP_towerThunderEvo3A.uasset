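; Evolution 3A of the thunder tower in a tower defense, firing Projectile_Feu at jomviking1 enemies.
; BeginPlay loads mesh, range, damage and fire rate from StatsTours row "Table_electrique".
; Sphere overlaps set or clear the target; Tick shoots or runs a throttled closest-target trace, whose result clears Towertarget instead of assigning it.
; Clicking toggles the tower widget; selling destroys the actor and removes it.
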(event OnComponentEndOverlap(Sphere)
  (params (OverlappedComponent :type Primitive%20Component%20Object%20Reference) (OtherActor :type Actor%20Object%20Reference) (OtherComp :type Primitive%20Component%20Object%20Reference) (OtherBodyIndex :type Integer))
  (Utilities|FlowControl|Sequence
    (:then_0
      (if (== (Variables|Default|GetTowertarget) OtherActor)
        (Variables|Default|SetTowertarget 0)))
    (:then_1
      (if (== (Variables|Default|GetTowertarget2) OtherActor)
        (Variables|Default|SetTowertarget2 0)))))

(event OnComponentBeginOverlap(Sphere)
  (params (OverlappedComponent :type Primitive%20Component%20Object%20Reference) (OtherActor :type Actor%20Object%20Reference) (OtherComp :type Primitive%20Component%20Object%20Reference) (OtherBodyIndex :type Integer) (bFromSweep :type Boolean) (SweepResult :type Hit%20Result%20Structure%20%28by%20ref%29))
  (Utilities|IsValid (Variables|Default|GetTowertarget)
    (:Is%20Not%20Valid
      (bind _asjomviking_1 (Utilities|Casting|CastTojomviking1 OtherActor))
      (Variables|Default|SetTowertarget _asjomviking_1))))

(event Custom|TowerInit
  (bind _towerstruct (Variables|Default|GetTowerStruct))
  (bind (_nom _portée _degats _firerate _mesh) (Utilities|Struct|BreakTowerStruct _towerstruct))
  (Components|StaticMesh|SetStaticMesh (Variables|Default|GetCube) _mesh)
  (Components|Sphere|SetSphereRadius (Variables|Default|GetSphere) _portée true))

(event Custom|sellTowerThunder3A
  ;[1 1 1] Sell tower thunder evo 3A
  (Actor|DestroyActor)
  ;[1 1 1] Ouverture/fermeture du widget
  (Widget|RemovefromParent (stale MouseInput|EventActorOnClicked _returnvalue)))

(event Custom|shoot
  (bind _towerstruct (Variables|Default|GetTowerStruct))
  (bind (_nom _portée _degats _firerate) (Utilities|Struct|BreakTowerStruct _towerstruct))
  ;[1 1 1] Modifier quand il y aura les ennemis
  (Variables|Default|Setreload true)
  (Game|SpawnActorfromClass "/Game/Tours/Projectile_Feu.Projectile_Feu_C" (Transformation|GetActorTransform) "AlwaysSpawn" 0 (Variables|Default|GetTowertarget) _degats 0)
  (Utilities|FlowControl|Delay _firerate)
  (Variables|Default|Setreload false))

(event Custom|SelectNewTarget
  (bind _returnvalue (Transformation|GetActorLocation))
  (Variables|Default|SetCheckForTarget true)
  (bind _outhits (Collision|MultiSphereTraceForObjects _returnvalue (- _returnvalue "0, 0, 0") (.Portée (Utilities|Struct|BreakTowerStruct (Variables|Default|GetTowerStruct))) (Utilities|Array|MakeArray "ObjectTypeQuery3") false 0 "None"))
  (if true
    (bind _ennemies (CallFunction|CloserTarget _outhits))
    (Utilities|IsValid _ennemies
      (:Is%20Valid
        (Variables|Default|SetTowertarget 0))
      (:Is%20Not%20Valid
        _)))
  (Utilities|FlowControl|Delay 0.2)
  (Variables|Default|SetCheckForTarget false))

(event EventBeginPlay
  (bind _returnvalue (Utilities|GetDataTableRow "/Game/Tours/StatsTours.StatsTours" "Table_electrique")
    (:then
      (Variables|Default|SetTowerStruct _returnvalue)
      (CallFunction|TowerInit))))

(event MouseInput|EventActorOnClicked
  (params (ButtonPressed :type Key%20Structure :default "None"))
  ;[1 1 1] Ouverture/fermeture du widget
  (Utilities|FlowControl|FlipFlop
    (:A
      (bind _returnvalue (UserInterface|CreateWidget "/Game/Tours/towerThunder/widgetTowerThunderEvo3A.widgetTowerThunderEvo3A_C"))
      (UserInterface|Viewport|AddtoViewport _returnvalue 0))
    (:B
      (Widget|RemovefromParent _returnvalue))))

(event EventTick
  (params (DeltaSeconds :type Float%20%28single-precision%29))
  (Utilities|IsValid (Variables|Default|GetTowertarget)
    (:Is%20Valid
      (if (not (Variables|Default|Getreload))
        (CallFunction|Shoot)))
    (:Is%20Not%20Valid
      (if (not (Variables|Default|GetCheckForTarget))
        (CallFunction|SelectNewTarget)))))

(fn ConstructionScript)

(fn CloserTarget
  (params (Array :type Array%20of%20Hit%20Result%20Structures))
  ;[1 1 1] Modifier quand il y aura les ennemis
  (for _array_element Array
    (bind _asjomviking_1 (Utilities|Casting|CastTojomviking1 (.HitActor (Collision|BreakHitResult _array_element))))
    (Utilities|IsValid (LocalVariables|GetIs%20a%20Target?)
      (:Is%20Valid
        (if (< (Math|Vector|VectorLength (- (Transformation|GetActorLocation) (Transformation|GetActorLocation (.HitActor (Collision|BreakHitResult _array_element))))) (Variables|Default|Getdistance%20temp))
          (LocalVariables|SetIs%20a%20Target? _asjomviking_1)
          (Variables|Default|Setdistance%20temp (Math|Vector|VectorLength (- (Transformation|GetActorLocation) (Transformation|GetActorLocation (.HitActor (Collision|BreakHitResult _array_element))))))))
      (:Is%20Not%20Valid
        (LocalVariables|SetIs%20a%20Target? _asjomviking_1)
        (Variables|Default|Setdistance%20temp (Math|Vector|VectorLength (- (Transformation|GetActorLocation) (Transformation|GetActorLocation (.HitActor (Collision|BreakHitResult _array_element)))))))))
  (return (LocalVariables|GetIs%20a%20Target?)))